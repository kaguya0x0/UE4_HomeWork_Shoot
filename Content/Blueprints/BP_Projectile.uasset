(event Collision|EventHit
  (params (MyComp :type Primitive%20Component%20Object%20Reference) (Other :type Actor%20Object%20Reference) (OtherComp :type Primitive%20Component%20Object%20Reference) (bSelfMoved :type Boolean) (HitLocation :type Vector :default "0, 0, 0") (HitNormal :type Vector :default "0, 0, 0") (NormalImpulse :type Vector :default "0, 0, 0") (Hit :type Hit%20Result%20Structure%20%28by%20ref%29))
  (bind (_x _y) (Math|Vector|BreakVector HitLocation))
  (Utilities|Casting|CastToWall Other
    (:then
      (Audio|PlaySoundatLocation "/Game/Audio/hitMetal.hitMetal" HitLocation "0, 0, 0" 1.0 1.0 0.0 0 0 0)
      (Physics|AddForce (Variables|Default|GetStaticMesh1) (Math|Vector|MakeVector (* _x 0.4) (* _y 0.4) 0.0) "None" false)
      (Utilities|FlowControl|Delay 0.8)
      (Effects|SpawnEmitteratLocation "/Game/StarterContent/Particles/P_Explosion.P_Explosion" "0, 0, 0")
      (Audio|PlaySound2D "/Game/StarterContent/Audio/Explosion02.Explosion02" 1.0 1.0 0.0 0 0)
      (Actor|DestroyActor))
    (:CastFailed
      ;[0 1 0] Sound
      (Audio|PlaySoundatLocation "/Game/Sounds/SoundCue_Attentuated.SoundCue_Attentuated" HitLocation "0, 0, 0" (Variables|Default|GetVolumeMultiplier) (Math|Random|RandomFloatinRange 0.8 1.2) 0.0 0 0 0)
      (Utilities|Casting|CastToCharacter Other
        (:then
          (if (Components|ComponentHasTag OtherComp "Hat")
            ;[1 1 1] Hit Hat
            (Actor|DestroyActor)
            (Physics|SetSimulatePhysics OtherComp true)
            (Physics|SetPhysicsLinearVelocity OtherComp (/ (Variables|/Script/Engine.MovementComponent|GetVelocity (Variables|Default|GetProjectileMovement)) 3.0) false "None")
            (Class|PrimitiveComponent|SetPhysicsAngularVelocityinDegrees OtherComp (Math|Vector|MakeVector (Math|Random|RandomFloatinRange -7.2e+02 7.2e+02) (Math|Random|RandomFloatinRange -7.2e+02 7.2e+02) (Math|Random|RandomFloatinRange -7.2e+02 7.2e+02)) false "None")
            ;[0 1 0] Sound
            (Audio|PlaySoundatLocation "/Game/Sounds/Randomize_01.Randomize_01" HitLocation "0, 0, 0" (* (Variables|Default|GetVolumeMultiplier) 0.25) 1.0 0.0 0 0 0)
            (else
              ;[1 1 1] Hit Character
              (Game|Damage|ApplyDamage Other (Math|Random|RandomFloatinRange 1.1e+02 1.1e+02) (Game|GetInstigatorController) self)
              (Actor|DestroyActor :!label _label)
              (Effects|SpawnEmitteratLocation "/Game/Effects/P_Hit.P_Hit" HitLocation))))
        (:CastFailed
          (bind _asfly_cube (Utilities|Casting|CastToFlyCube Other)
            (:then
              (Default|CubeGetHit _asfly_cube (Variables|组件|GetcurrentPlayer))
              (Actor|DestroyActor)
              (Effects|SpawnEmitteratLocation "/Game/StarterContent/Particles/P_Fire.P_Fire" HitLocation "0, 0, 0" "1.000000,1.000000,1.000000" false)
              (Audio|PlaySoundatLocation "/Game/StarterContent/Audio/Collapse01.Collapse01" HitLocation "0, 0, 0" 1.0 1.0 0.0 0 0 0)
              (Utilities|FlowControl|Delay 0.8)
              (Actor|DestroyActor Other)
              (Utilities|FlowControl|Delay 0.2))
            (:CastFailed
              (goto _label))))))))

(fn ConstructionScript)